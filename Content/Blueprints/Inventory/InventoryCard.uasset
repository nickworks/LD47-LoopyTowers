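; Inventory card that stores an action type (Aim, Shoot, TurnCW, TurnCCW, Reload), its power and a name taken from the type.
; Random initialization picks a type and rolls a rareness bounded by the player's RarenessBuff.
; Rareness indexes clamped per-type power tables, with an extra random offset for Shoot and Reload.
; Aim's table index is fixed at zero, so its power is always 1.
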(fn `Initialize Card`
  (params (`Card Type` :type "/Game/Blueprints/Inventory/CardTypes Enum" :default "NewEnumerator0") (Power :type Integer))
  (set `self.card type` `Card Type`)
  (set `self.card power` Power)
  (set `self.name` (`|GetEnumeratorNameAsString` (`self.card type`))))

(fn `Initialize Random Card`
  (params (Player :type "/Game/Blueprints/Player/TopDownController Object Reference"))
  (locals (`Temp Type` :type "/Game/Blueprints/Inventory/CardTypes Enum"))
  (bind _returnvalue (select `int` (`KismetMathLibrary.Clamp` (`self.rareness`) 0 10) :`0` 90 :`1` 90 :`2` 180 :`3` 180 :`4` 45 :`5` 45 :`6` 135 :`7` 120 :`8` 120 :`9` 60 :`10` 30))
  (set `self.rareness` (`KismetMathLibrary.RandomInteger` (`/Game/Blueprints/Player/TopDownController.rareness buff` Player)))
  (set `local.Temp Type` (cast `/Game/Blueprints/Inventory/CardTypes` (`KismetMathLibrary.Conv_IntToByte` (`KismetMathLibrary.RandomInteger` (enumcount `/Game/Blueprints/Inventory/CardTypes`)))))
  (`self.Initialize Card` (`local.Temp Type`) (select `/Game/Blueprints/Inventory/CardTypes` (`local.Temp Type`) :`NewEnumerator0` (select `int` 0 :`0` 1 :`1` 1 :`2` 2 :`3` 2 :`4` 3 :`5` 3 :`6` 4 :`7` 5 :`8` 8 :`9` 9 :`10` 10 :`11` 12 :`12` 13 :`13` 14 :`14` 100) :`NewEnumerator1` (select `int` (`KismetMathLibrary.Clamp` (+ (`KismetMathLibrary.RandomIntegerInRange` 0 4) (`self.rareness`)) 0 14) :`0` 1 :`1` 1 :`2` 2 :`3` 2 :`4` 3 :`5` 3 :`6` 4 :`7` 5 :`8` 8 :`9` 9 :`10` 10 :`11` 12 :`12` 13 :`13` 14 :`14` 15) :`NewEnumerator2` _returnvalue :`NewEnumerator3` _returnvalue :`NewEnumerator5` (select `int` (`KismetMathLibrary.Clamp` (+ (`KismetMathLibrary.RandomIntegerInRange` 0 3) (`self.rareness`)) 0 13) :`0` 1 :`1` 2 :`2` 3 :`3` 4 :`4` 5 :`5` 6 :`6` 7 :`7` 8 :`8` 9 :`9` 10 :`10` 15 :`11` 20 :`12` 30 :`13` 50))))