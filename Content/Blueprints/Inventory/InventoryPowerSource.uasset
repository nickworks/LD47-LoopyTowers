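; Inventory item Blueprint for a power source, holding its type, total fuel and remaining fuel.
; The initializer stores type and fuel amount and names the item after the enum entry, leaving its chamber size input unused.
; The random initializer picks a type, rolls rareness from the player controller's RarenessBuff, then passes a random fuel amount, bounded by rareness and scaled per type, to the base initializer.
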(fn `Initialize Power Source`
  (params (`Power Type` :type "/Game/Blueprints/Inventory/PowerSourceTypes Enum" :default "NewEnumerator0") (`Amount of Fuel` :type Integer) (`Chamber Size` :type Integer :default 5))
  (set `self.power source type` `Power Type`)
  (set `self.total fuel` `Amount of Fuel`)
  (set `self.how much fuel is left` `Amount of Fuel`)
  (set `self.name` (`|GetEnumeratorNameAsString` (`self.power source type`))))

(fn `Initialize Random Power Source`
  (params (`Player Controller` :type "/Game/Blueprints/Player/TopDownController Object Reference"))
  (locals (`temp type` :type "/Game/Blueprints/Inventory/PowerSourceTypes Enum") (rareness :type Integer))
  (bind _returnvalue (`KismetMathLibrary.RandomIntegerInRange` 1 (+ (`local.rareness`) 1)))
  (set `local.rareness` (`KismetMathLibrary.RandomInteger` (`/Game/Blueprints/Player/TopDownController.rareness buff` `Player Controller`)))
  (set `local.temp type` (cast `/Game/Blueprints/Inventory/PowerSourceTypes` (`KismetMathLibrary.Conv_IntToByte` (`KismetMathLibrary.RandomInteger` (enumcount `/Game/Blueprints/Inventory/PowerSourceTypes`)))))
  (`self.Initialize Power Source` (`local.temp type`) (`KismetMathLibrary.FTrunc` (select `/Game/Blueprints/Inventory/PowerSourceTypes` (`local.temp type`) :`NewEnumerator1` (* _returnvalue 50.0) :`NewEnumerator2` (* _returnvalue 20.0) :`NewEnumerator3` (* _returnvalue 10.0) :`NewEnumerator4` (* _returnvalue 30.0) :`NewEnumerator5` (* _returnvalue 15.0)))))