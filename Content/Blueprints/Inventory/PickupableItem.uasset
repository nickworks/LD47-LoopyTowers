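; PickupableItem is a world pickup actor that shows a randomly generated inventory card on a floating widget.
; On BeginPlay it constructs an InventoryCard, initializes it through the TopDownController and passes it to the InventoryItem widget.
; A Hover timeline bobs and spins the widget.
; SetHoverState brightens the point light and enlarges the widget for highlighting.
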(event `self.ReceiveBeginPlay`
  (bind _widgetoffset (`self.WidgetOffset`))
  (`self.Random Item`)
  (bind (_direction _hover _spin) (`Timeline|Hover`)
    (:`Update`
      (`SceneComponent.K2_SetWorldLocation` _widgetoffset (+ (`KismetMathLibrary.MakeVector` 0.0 0.0 (* _hover 40.0)) (`self.K2_GetActorLocation`)) false false)
      (`SceneComponent.K2_SetWorldRotation` _widgetoffset (struct :`Pitch` 110.0) false false)
      (`SceneComponent.K2_SetRelativeRotation` (`self.Widget`) (`KismetMathLibrary.MakeRotator` (* _spin 360.0)) false false))))

(fn `Random Item`
  (bind _astop_down_controller (cast `/Game/Blueprints/Player/TopDownController` (`GameplayStatics.GetPlayerController` 0)))
  ;[1 1 1] Build Item: RANDOM Card
  (bind _returnvalue (`|GenericCreateObject` "/Game/Blueprints/Inventory/InventoryCard.InventoryCard_C" "/Game/Blueprints/Inventory/Inventory_Item.Inventory_Item"))
  (set `self.Inventory Item` _returnvalue)
  (`/Game/Blueprints/Inventory/InventoryCard.Initialize Random Card` _returnvalue _astop_down_controller)
  ;[1 1 1] Build Widget
  (bind _asinventory_item (cast `/Game/Blueprints/Widgets/InventoryItem` (`WidgetComponent.GetUserWidgetObject` (`self.Widget`))))
  (`/Game/Blueprints/Widgets/InventoryItem.Set Item DATA` _asinventory_item (`self.Inventory Item`)))

(fn `Set Hover State`
  (params (`Is On` :type Boolean))
  (`LightComponent.SetIntensity` (`self.PointLight`) (select `bool` `Is On` :`false` 1000.0 :`true` 5000.0 :!type "Float (single-precision)"))
  (`SceneComponent.SetRelativeScale3D` (`self.Widget`) (`KismetMathLibrary.Conv_DoubleToVector` (select `bool` `Is On` :`false` 0.5 :`true` 0.75 :!type "Float (single-precision)"))))

(fn `UserConstructionScript`)