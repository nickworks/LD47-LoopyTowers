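; Monster character that becomes a random MonsterDatabase row on BeginPlay, setting its scale, pixel-art sprite, bounce curve and puppet offset.
; Tick runs a cooldown-based Idle/Walking/Attacking state machine that targets the player pawn, walks over with AIMoveTo and attacks within range.
; Timelines animate the sprite puppet: walking bounces with randomized tilt and speed, while attacking lunges toward the target, with no damage applied here.
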(event `self.ReceiveBeginPlay`
  (bind _thing_i_want_to_attack (`self.Thing I want to attack`))
  (bind _returnvalue (`self.Get Random Monster Type`))
  (`self.Become Monster` _returnvalue)
  (bind (_direction _newtrack_0) (`Timeline|Attack Animation` :!via `SetNewTime`)
    (:`Update`
      (`/Engine/EditorBlueprintResources/StandardMacros.IsValid` _thing_i_want_to_attack
        (:`Is Valid`
          (`SceneComponent.K2_SetRelativeLocation` (`self.PuppetAttack`) (+ (* (`KismetMathLibrary.Normal` (- (`self.K2_GetActorLocation` _thing_i_want_to_attack) (`self.K2_GetActorLocation`))) (* _newtrack_0 50.0)) (`self.Offset PuppetAttack`)) false false))))))

(event `self.ReceiveTick`
  (params (DeltaSeconds :type "Float (single-precision)"))
  (bind _thing_i_want_to_attack (`self.Thing I want to attack`))
  (`self.Countdown cooldown` DeltaSeconds)
  (switch `/Game/Blueprints/MonsterState` (`self.CurrentState`)
    (:`NewEnumerator0`
      (`/Engine/EditorBlueprintResources/StandardMacros.IsValid` _thing_i_want_to_attack
        (:`Is Valid`
          (if (< (`self.GetDistanceTo` _thing_i_want_to_attack) (`self.Attack distance`))
            (`self.Attack`)
            (else
              ;[1 1 1] Walk towards target
              (bind _asaicontroller (cast `AIController` (`self.GetController`)))
              (`AITask_MoveTo.AIMoveTo` _asaicontroller (0.0 0.0 0.0) (`self.Thing I want to attack`) 100.0 "Default" "Default" true false
                (:`then`
                  (`self.Set Monster State` "NewEnumerator1" 5.0))
                (:`OnRequestFailed`
                  (`self.Set Monster State` "NewEnumerator0" :!label _label))
                (:`OnMoveFinished`
                  (goto _label))))))
        (:`Is Not Valid`
          (set `self.Thing I want to attack` (`GameplayStatics.GetPlayerPawn` 0)))))))

(fn `AnimateWalking`
  (`SceneComponent.K2_SetWorldRotation` :`self` (`self.PuppetROOT`)))

(fn `Attack`
  (bind _attack_animation (`self.Attack Animation`))
  (`self.Set Monster State` "NewEnumerator2" (`TimelineComponent.GetTimelineLength` _attack_animation))
  (`TimelineComponent.PlayFromStart` _attack_animation))

(fn `Become Monster`
  (params (MonsterType :type "/Game/Art/TeamMonsters/MonsterTypes Structure"))
  (locals (`Row Name` :type Name :default "RowOne") (`Dynamic Material` :type "MaterialInstanceDynamic Object Reference"))
  (bind (_monstertype_name _monstertype_sprite _monstertype_bounciness _monstertype_verticalmotion _monstertype_scale _monstertype_verticaloffset) (break `/Game/Art/TeamMonsters/MonsterTypes` (`local.MonsterType`)))
  (bind _walkinganimation (`self.WalkingAnimation`))
  (set `self.CurrentState` "NewEnumerator0")
  (bind _returnvalue (`PrimitiveComponent.CreateDynamicMaterialInstance` (`self.Pixel Art`) 0 "/Game/Art/TeamMonsters/MONSTER_MAT.MONSTER_MAT" "None"))
  (`SceneComponent.SetWorldScale3D` (`self.CapsuleComponent`) (`KismetMathLibrary.Conv_DoubleToVector` MonsterType_Scale_14_B113E46145B93C4E89ADECBF6BC4F0B4))
  (set `local.Dynamic Material` _returnvalue)
  (`MaterialInstanceDynamic.SetTextureParameterValue` (`local.Dynamic Material`) "Sprite" MonsterType_Sprite_5_6BE83F664C6C7E913247CF9AD333F6AD)
  (`TimelineComponent.SetFloatCurve` _walkinganimation MonsterType_VerticalMotion_11_4E5B27D44C1F092E2F64109B52814BB3 "Bouncy")
  (`TimelineComponent.PlayFromStart` _walkinganimation)
  (bind _output_get (set `self.Offset PuppetAttack` (`KismetMathLibrary.MakeVector` 0.0 0.0 (+ _monstertype_verticaloffset 100.0))))
  (`SceneComponent.K2_SetRelativeLocation` (`self.PuppetAttack`) _output_get false false))

(fn `Countdown cooldown`
  (params (DT :type "Float (double-precision)"))
  (if (> (`self.cooldown`) 0.0)
    (set `self.cooldown` (- (`self.cooldown`) DT))
    (else
      (set `self.CurrentState` "NewEnumerator0"))))

(fn `Get Random Monster Type`
  (returns (ReturnValue :type "/Game/Art/TeamMonsters/MonsterTypes Structure"))
  (bind _outrownames (`DataTableFunctionLibrary.GetDataTableRowNames` "/Game/Art/TeamMonsters/MonsterDatabase.MonsterDatabase"))
  (bind _returnvalue (`|GetDataTableRow` "/Game/Art/TeamMonsters/MonsterDatabase.MonsterDatabase" (`|GetArrayItem` _outrownames (`KismetMathLibrary.RandomInteger` (`KismetArrayLibrary.Array_Length` _outrownames))))
    (:`then`
      (return _returnvalue))))

(fn `Set Monster State`
  (params (`New state` :type "/Game/Blueprints/MonsterState Enum" :default "NewEnumerator0") (`Minimum cooldown` :type "Float (double-precision)"))
  (bind _output_get (set `self.CurrentState` `New state`))
  (bind _output_get_2 (set `self.cooldown` `Minimum cooldown`)))

(fn `UserConstructionScript`)