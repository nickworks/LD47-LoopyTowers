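; Pickupable item actor that holds a randomly generated inventory card and shows a hovering, spinning widget in the world.
; On BeginPlay, RandomItem constructs an InventoryCard, stores it as InventoryItem and initializes it randomly with the player's TopDownController.
; The Hover timeline then lifts the widget's offset component above the actor at a fixed world rotation and rolls the widget.
; The file contains no overlap or pickup logic.
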(event `self.ReceiveBeginPlay`
  (bind _widgetoffset (`self.WidgetOffset`))
  (`self.Random Item`)
  (bind (_direction _hover _spin) (`Timeline|Hover`)
    (:`Update`
      (`SceneComponent.K2_SetWorldLocation` _widgetoffset (+ (`KismetMathLibrary.MakeVector` 0.0 0.0 (* _hover 40.0)) (`self.K2_GetActorLocation`) (0.0 0.0 0.0)) false false)
      (`SceneComponent.K2_SetWorldRotation` _widgetoffset (struct :`Pitch` 110.0) false false)
      (`SceneComponent.K2_SetRelativeRotation` (`self.Widget`) (`KismetMathLibrary.MakeRotator` (* _spin 360.0)) false false))))

(fn `Random Item`
  (bind _astop_down_controller (cast `/Game/Blueprints/TopDownController` (`GameplayStatics.GetPlayerController` 0)))
  (bind _returnvalue (`|GenericCreateObject` "/Game/Blueprints/Widgets/InventoryCard.InventoryCard_C" "/Game/Blueprints/Widgets/Inventory_Item.Inventory_Item"))
  (set `self.Inventory Item` _returnvalue)
  (`/Game/Blueprints/Widgets/InventoryCard.Initialize Random Card` _returnvalue _astop_down_controller))

(fn `UserConstructionScript`)