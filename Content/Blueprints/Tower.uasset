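; Tower actor that the player can hover and select to manage its card slots and power source.
; Hover events toggle a highlight material parameter on RoboArt.
; Selection opens a MenuTower widget in UI-only input, whose update event writes back the tower's slots and passes inventory to TopDownController.
; Closing removes the menu, notifies the controller and forces garbage collection; radius bubble scaling logic is unconnected.
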(event `Begin Hover`
  (`MeshComponent.SetScalarParameterValueOnMaterials` (`self.Robo Art`) "Highlight Amount" 1.0)
  (`KismetSystemLibrary.PrintString` "Hello"))

(event `End Hover`
  (`MeshComponent.SetScalarParameterValueOnMaterials` (`self.Robo Art`) "Highlight Amount" 0.0))

(event `On Selected by Player`
  (bind _returnvalue (`|CreateWidget` "/Game/Blueprints/Widgets/MenuTower.MenuTower_C"))
  (bind _output_get (set `self.MENU` _returnvalue))
  (`/Game/Blueprints/Widgets/MenuTower.Build Tower Inventory` _output_get self)
  (`/Game/Blueprints/Widgets/MenuTower.After Initial Build` _output_get)
  (add `/Game/Blueprints/Widgets/MenuTower.Close Menu` _output_get (delegate `Tower Menu Closed`))
  (add `/Game/Blueprints/Widgets/MenuTower.Items Get Updated` _output_get (delegate `Menu Items Updated`))
  (`UserWidget.AddToViewport` _output_get 0)
  (`WidgetBlueprintLibrary.SetInputMode_UIOnlyEx` (`GameplayStatics.GetPlayerController` 0) null))

(event `Menu Items Updated`
  (params (`Cards in Tower` :type "Array of /Game/Blueprints/Widgets/InventoryCard Object Reference (by ref)") (`Power Source in Tower` :type "/Game/Blueprints/Widgets/InventoryPowerSource Object Reference") (`Inventory Items` :type "Array of /Game/Blueprints/Widgets/Inventory_Item Object Reference (by ref)"))
  (set `self.Card Slots` `Cards in Tower`)
  (set `self.Power Source Slot` `Power Source in Tower`)
  (bind _astop_down_controller (cast `/Game/Blueprints/TopDownController` (`GameplayStatics.GetPlayerController` 0)))
  (`/Game/Blueprints/TopDownController.Inventory - SET` _astop_down_controller `Inventory Items`))

(event `Tower Menu Closed`
  (`Widget.RemoveFromParent` (`self.MENU`))
  (set `self.MENU` null)
  (bind _astop_down_controller (cast `/Game/Blueprints/TopDownController` (`GameplayStatics.GetPlayerController` 0)))
  (`/Game/Blueprints/TopDownController.On Close Tower Menu` _astop_down_controller)
  (`KismetSystemLibrary.CollectGarbage`))

(fn `UserConstructionScript`)