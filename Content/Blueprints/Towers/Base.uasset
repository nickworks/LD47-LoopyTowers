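; Tower base Blueprint with a generator sphere and six LED components that serve as selectable goal points.
; On BeginPlay it sets the sphere materials' Glow Amount parameter to switch on the glow.
; Pick LED GOAL returns the world location of a randomly chosen LED.
; A ForEachWithDelay macro steps through an index range with a delay between iterations, though no graph here calls it.
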(event `self.ReceiveBeginPlay`
  (`MeshComponent.SetScalarParameterValueOnMaterials` (`self.Generator Sphere`) "Glow Amount" 1.0))

(fn `Pick LED GOAL`
  (returns (NewParam :type "Vector Structure"))
  (bind _array (`|MakeArray` (`self.LED 06`) (`self.LED 02`) (`self.LED 04`) (`self.LED 03`) (`self.LED 01`) (`self.LED 05`)))
  (return (`SceneComponent.K2_GetComponentLocation` (`|GetArrayItem` _array (`KismetMathLibrary.RandomInteger` (`KismetArrayLibrary.Array_Length` _array))))))

(fn `UserConstructionScript`)