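; Programmable tower that acts as a solid wall until a power source is slotted, then becomes a robot turret with art matching the power type.
; Each Tick advances through a randomly sized loop of card slots, running Shoot, Turn or Reload cards scaled by card power.
; Reload draws ammo from the power source's fuel, and Shoot spends it on delayed bursts.
; A UMG menu edits slots and inventory via bound events.
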(event `self.ReceiveBeginPlay`
  (bind _returnvalue (`PrimitiveComponent.CreateDynamicMaterialInstance` (`self.Robo Art`) 0 "/Game/Art/TeamBots/BOT_MAT.BOT_MAT" "None"))
  (set `self.ROBOT dynamic material` _returnvalue)
  (`self.Update View`)
  (set `self.Ammo Capacity` (* (`KismetMathLibrary.RandomIntegerInRange` 1 5) 5))
  (bind _output_get (set `self.Number of Card Slots` (`KismetMathLibrary.RandomIntegerInRange` 3 6)))
  (for _ (range (+ _output_get 1))
    (`KismetArrayLibrary.Array_Add` (`self.Card Slots`))))

(event `On Selected by Player`
  (bind _returnvalue (`|CreateWidget` "/Game/Blueprints/Widgets/MenuTower.MenuTower_C"))
  (bind _output_get (set `self.MENU` _returnvalue))
  (`/Game/Blueprints/Widgets/MenuTower.Build Tower Inventory` _output_get self)
  (`/Game/Blueprints/Widgets/MenuTower.After Initial Build` _output_get)
  (add `/Game/Blueprints/Widgets/MenuTower.Close Menu` _output_get (delegate `Tower Menu Closed`))
  (add `/Game/Blueprints/Widgets/MenuTower.Items Get Updated` _output_get (delegate `Menu Items Updated`))
  (`UserWidget.AddToViewport` _output_get 0)
  (`WidgetBlueprintLibrary.SetInputMode_UIOnlyEx` (`GameplayStatics.GetPlayerController` 0) null))

(event `Menu Items Updated`
  (params (`Cards in Tower` :type "Array of /Game/Blueprints/Inventory/InventoryCard Object Reference (by ref)") (`Power Source in Tower` :type "/Game/Blueprints/Inventory/InventoryPowerSource Object Reference") (`Inventory Items` :type "Array of /Game/Blueprints/Inventory/Inventory_Item Object Reference (by ref)"))
  (set `self.Card Slots` `Cards in Tower`)
  (set `self.Power Source Slot` `Power Source in Tower`)
  (bind _astop_down_controller (cast `/Game/Blueprints/Player/TopDownController` (`GameplayStatics.GetPlayerController` 0)))
  (`/Game/Blueprints/Player/TopDownController.Inventory - SET` _astop_down_controller `Inventory Items`)
  (`self.Update View`))

(event `Tower Menu Closed`
  (`Widget.RemoveFromParent` (`self.MENU`))
  (set `self.MENU` null)
  (bind _astop_down_controller (cast `/Game/Blueprints/Player/TopDownController` (`GameplayStatics.GetPlayerController` 0)))
  (`/Game/Blueprints/Player/TopDownController.On Close Tower Menu` _astop_down_controller)
  (`KismetSystemLibrary.CollectGarbage`))

(event `CardAbilityShoot`
  (params (`Amount of Projectiles` :type Integer) (`Delay between Shots` :type "Float (double-precision)"))
  (bind _menu (`self.MENU`))
  ;[1 1 1] Shoot
  (`self.ForEachWithDelay` 0 (- `Amount of Projectiles` 1) `Delay between Shots`
    (:`Loop Body`
      (if (> (`self.Ammo Loaded`) 0)
        (`self.Shoot Projectile`)
        (`/Engine/EditorBlueprintResources/StandardMacros.DecrementInt` (`self.Ammo Loaded`)
          (:`  `
            (`/Engine/EditorBlueprintResources/StandardMacros.IsValid` _menu
              (:`Is Valid`
                (`/Game/Blueprints/Widgets/MenuTower.Update Fuel` _menu self)))))))))

(event `self.ReceiveTick`
  (params (DeltaSeconds :type "Float (single-precision)"))
  (bind (_relativerotation_roll _relativerotation_pitch _relativerotation_yaw) (`KismetMathLibrary.BreakRotator` (`SceneComponent.RelativeRotation` (`self.Aim Swivel`))))
  (bind _card_power (`/Game/Blueprints/Inventory/InventoryCard.card power` (`self.Active Card`)))
  (bind _returnvalue (`KismetMathLibrary.Conv_IntToDouble` (`/Game/Blueprints/Inventory/InventoryCard.card power` (`self.Active Card`))))
  (`/Engine/EditorBlueprintResources/StandardMacros.IsValid` (`self.Power Source Slot`)
    (:`Is Valid`
      (`self.Step to Next Card`)
      (`self.Move MENU Active Highlight`)
      ;[1 1 1] Activate current card
      (bind _output_get (set `self.Active Card` (`|GetArrayItem` (`self.Card Slots`) (`self.current card index`))))
      (`/Engine/EditorBlueprintResources/StandardMacros.IsValid` _output_get
        (:`Is Valid`
          (switch `/Game/Blueprints/Inventory/CardTypes` (`/Game/Blueprints/Inventory/InventoryCard.card type` (`self.Active Card`))
            (:`NewEnumerator1`
              (`self.CardAbilityShoot` _card_power (/ 1.0 (`KismetMathLibrary.Conv_IntToDouble` _card_power))))
            (:`NewEnumerator2`
              ;[1 1 1] Spin
              (set `self.Anim Rotation End` (+ _relativerotation_yaw _returnvalue))
              (set `self.Anim Rotation Start` _relativerotation_yaw :!label _label)
              (bind (_direction _percent_complete) (`Timeline|Rotation` :!via `PlayFromStart`)
                (:`Update`
                  (`SceneComponent.K2_SetRelativeRotation` (`self.Aim Swivel`) (`KismetMathLibrary.MakeRotator` 0.0 0.0 (`KismetMathLibrary.Lerp` (`self.Anim Rotation Start`) (`self.Anim Rotation End`) _percent_complete)) true false))))
            (:`NewEnumerator3`
              (set `self.Anim Rotation End` (- _relativerotation_yaw _returnvalue))
              (goto _label))
            (:`NewEnumerator5`
              (`self.Reload`))))))))

(fn `Move MENU Active Highlight`
  (bind _menu (`self.MENU`))
  (`/Engine/EditorBlueprintResources/StandardMacros.IsValid` _menu
    (:`Is Valid`
      (`/Game/Blueprints/Widgets/MenuTower.Update Active Highlight` _menu self))))

(fn `Reload`
  (locals (`Number to Draw` :type Integer :default 0))
  (bind _menu (`self.MENU`))
  (bind _power_source_slot (`self.Power Source Slot`))
  (bind _how_much_fuel_is_left (`/Game/Blueprints/Inventory/InventoryPowerSource.how much fuel is left` _power_source_slot))
  (`/Engine/EditorBlueprintResources/StandardMacros.IsValid` _power_source_slot
    (:`Is Valid`
      (bind _output_get (set `local.Number to Draw` (`KismetMathLibrary.Clamp` (`/Game/Blueprints/Inventory/InventoryCard.card power` (`self.Active Card`)) 0 (`KismetMathLibrary.Min` (- (`self.Ammo Capacity`) (`self.Ammo Loaded`)) _how_much_fuel_is_left))))
      (set `self.Ammo Loaded` (+ _output_get (`self.Ammo Loaded`)))
      (set `/Game/Blueprints/Inventory/InventoryPowerSource.how much fuel is left` (- _how_much_fuel_is_left (`local.Number to Draw`)) _power_source_slot)
      (`/Engine/EditorBlueprintResources/StandardMacros.IsValid` _menu
        (:`Is Valid`
          (`/Game/Blueprints/Widgets/MenuTower.Update Fuel` _menu self))))))

(fn `Set Hover`
  (params (`Is On` :type Boolean))
  (`MeshComponent.SetScalarParameterValueOnMaterials` (`self.LED 06`) "Glow Amount" (select `bool` `Is On` :`true` 1.0 :!type "Float (single-precision)"))
  (`MeshComponent.SetScalarParameterValueOnMaterials` (`self.LED 02`) "Glow Amount" (select `bool` `Is On` :`true` 1.0 :!type "Float (single-precision)"))
  (`MeshComponent.SetScalarParameterValueOnMaterials` (`self.LED 04`) "Glow Amount" (select `bool` `Is On` :`true` 1.0 :!type "Float (single-precision)"))
  (`MeshComponent.SetScalarParameterValueOnMaterials` (`self.LED 03`) "Glow Amount" (select `bool` `Is On` :`true` 1.0 :!type "Float (single-precision)"))
  (`MeshComponent.SetScalarParameterValueOnMaterials` (`self.LED 01`) "Glow Amount" (select `bool` `Is On` :`true` 1.0 :!type "Float (single-precision)"))
  (`MeshComponent.SetScalarParameterValueOnMaterials` (`self.LED 05`) "Glow Amount" (select `bool` `Is On` :`true` 1.0 :!type "Float (single-precision)"))
  (`MeshComponent.SetScalarParameterValueOnMaterials` (`self.Generator`) "Glow Amount" (select `bool` `Is On` :`true` 1.0 :!type "Float (single-precision)"))
  (`MeshComponent.SetScalarParameterValueOnMaterials` (`self.Robo Art`) "Highlight Amount" (select `bool` `Is On` :`true` 1.0 :!type "Float (single-precision)"))
  (`SceneComponent.SetWorldScale3D` (`self.Robo Art`) (`KismetMathLibrary.Conv_DoubleToVector` (select `bool` `Is On` :`false` 2.0 :`true` 3.0 :!type "Float (single-precision)")))
  (return))

(fn `Shoot Projectile`
  (bind (_returnvalue_location _returnvalue_rotation) (`KismetMathLibrary.BreakTransform` (`SceneComponent.K2_GetComponentToWorld` (`self.Arrow`))))
  (`|SpawnActorFromClass` "/Game/Blueprints/Towers/Projectile.Projectile_C" (`KismetMathLibrary.MakeTransform` _returnvalue_location _returnvalue_rotation) "Undefined" "OverrideRootScale" null null))

(fn `Step to Next Card`
  (bind _current_card_index (`self.current card index`))
  ;[1 1 1] Step to next card
  (`/Engine/EditorBlueprintResources/StandardMacros.IncrementInt` _current_card_index
    (:`  `
      (if (>= _current_card_index (`KismetArrayLibrary.Array_Length` (`self.Card Slots`)))
        (set `self.current card index` 0)))))

(fn `Update View`
  (bind _wall (`self.WALL`))
  (bind _is_turned_on (`self.Is Turned On`))
  (set `self.Is Turned On` (`KismetSystemLibrary.IsValid` (`self.Power Source Slot`)))
  (`SceneComponent.SetVisibility` (`self.Robo Art`) (`self.Is Turned On`) false)
  (`SceneComponent.SetVisibility` _wall (not _is_turned_on) false)
  (`PrimitiveComponent.SetCollisionEnabled` _wall (select `bool` _is_turned_on :`false` "QueryAndPhysics" :`true` "NoCollision" :!type "ECollisionEnabled Enum"))
  (`SceneComponent.SetVisibility` (`self.Gun`) (`self.Is Turned On`) true)
  (if (`self.Is Turned On`)
    (`MaterialInstanceDynamic.SetTextureParameterValue` (`self.ROBOT dynamic material`) "Sprite" (select `/Game/Blueprints/Inventory/PowerSourceTypes` (`/Game/Blueprints/Inventory/InventoryPowerSource.power source type` (`self.Power Source Slot`)) :`NewEnumerator1` "/Game/Art/TeamBots/bot-fire.bot-fire" :`NewEnumerator2` "/Game/Art/TeamBots/bot-gem.bot-gem" :`NewEnumerator3` "/Game/Art/TeamBots/bot-skull.bot-skull" :`NewEnumerator4` "/Game/Art/TeamBots/bot-dragon.bot-dragon" :`NewEnumerator5` "/Game/Art/TeamBots/bot-water.bot-water" :!type "Texture Object Reference"))))

(fn `UserConstructionScript`)